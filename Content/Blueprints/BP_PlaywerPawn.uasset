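; BP_PlaywerPawn is a player pawn that moves by applying torque to its static mesh, in the manner of a rolling object.
; Forward/backward and left/right axis inputs add torque around Y and X respectively, scaled by TorqueStrenght and applied as acceleration change, so mass is ignored.
; On BeginPlay it fades the player camera in from full opacity over a few seconds.
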(event `InputAxis|Move Forward/Backwards`
  (params (AxisValue :type "Float (single-precision)"))
  (`PrimitiveComponent.AddTorqueInRadians` (`self.StaticMesh`) (`KismetMathLibrary.MakeVector` 0.0 (* AxisValue (`self.Torque Strenght`))) "None" true))

(event `InputAxis|Move Left/Righ`
  (params (AxisValue :type "Float (single-precision)"))
  (`PrimitiveComponent.AddTorqueInRadians` (`self.StaticMesh`) (`KismetMathLibrary.MakeVector` (* AxisValue (`self.Torque Strenght`))) "None" true))

(event `self.ReceiveBeginPlay`
  (`PlayerCameraManager.StartCameraFade` :`self` (`GameplayStatics.GetPlayerCameraManager` 0) :`FromAlpha` 1.0 :`Duration` 3.0))

(fn `UserConstructionScript`)