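; BP_Cannon is a cannon actor that automatically fires projectiles on a repeating loop from BeginPlay.
; Each cycle waits for the RatFire delay, spawns a BP_Projectile at SpawnPoint scaled by ScaleProp, then plays CannonFireTimeline, whose completion restarts the cycle.
; The timeline drives the barrel's relative Y through a Lerp that unusually uses the barrel's world Y as its alpha.
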(event `self.ReceiveBeginPlay`
  (`KismetSystemLibrary.Delay` (`self.RatFire`) :!label _label)
  (`self.SpawnProjectile`)
  (bind (_direction _cannonbarrely_location) (`Timeline|Cannon Fire Timeline` :!via `PlayFromStart`)
    (:`Update`
      (`self.Barrel Y Animation` _cannonbarrely_location))
    (:`Finished`
      (goto _label))))

(fn `Barrel Y Animation`
  (params (`Cannon Barrel Y Location` :type "Float (double-precision)"))
  (bind (_returnvalue_x _returnvalue_y) (`KismetMathLibrary.BreakVector` (`SceneComponent.K2_GetComponentLocation` (`self.Cannon_Barrel`))))
  (`SceneComponent.K2_SetRelativeLocation` (`self.Cannon_Barrel`) (`KismetMathLibrary.MakeVector` 0.0 (`KismetMathLibrary.Lerp` `Cannon Barrel Y Location` 0.0 _returnvalue_y)) false false))

(fn `SpawnProjectile`
  (`|SpawnActorFromClass` "/Game/Blueprints/Projectiles/BP_Projectile.BP_Projectile_C" (`KismetMathLibrary.MakeTransform` (`SceneComponent.K2_GetComponentLocation` (`self.SpawnPoint`)) (`SceneComponent.K2_GetComponentRotation` (`self.SpawnPoint`)) (`KismetMathLibrary.Conv_DoubleToVector` (`self.ScaleProp`))) "AlwaysSpawn" "OverrideRootScale" null null))

(fn `UserConstructionScript`)