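; BP_Projectile is a projectile that hurts the player on contact and disappears when it overlaps any actor.
; The Sphere's begin-overlap event applies a small amount of damage and prints an "AŁA!" debug message only if the other actor is player pawn 0.
; Both branches then call DesstroyProjectile, which destroys the Sphere and Sphere1 components but leaves the actor itself alive.
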(event `self.Sphere.OnComponentBeginOverlap`
  (params (OverlappedComponent :type "PrimitiveComponent Object Reference") (OtherActor :type "Actor Object Reference") (OtherComp :type "PrimitiveComponent Object Reference") (OtherBodyIndex :type Integer) (bFromSweep :type Boolean) (SweepResult :type "HitResult Structure (by ref)"))
  (if (!= OtherActor (`GameplayStatics.GetPlayerPawn` 0))
    (`self.DesstroyProjectile`)
    (else
      (`GameplayStatics.ApplyDamage` (`GameplayStatics.GetPlayerPawn` 0) 0.1)
      (`KismetSystemLibrary.PrintString` "AŁA!" true false (struct :`R` 1.0 :`B` 0.476178 :`A` 1.0) 0.5)
      (`self.DesstroyProjectile`))))

(fn `DesstroyProjectile`
  (`ActorComponent.K2_DestroyComponent` (`self.Sphere1`))
  (`ActorComponent.K2_DestroyComponent` (`self.Sphere`)))

(fn `UserConstructionScript`)