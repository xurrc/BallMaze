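; Collectible crystal that flies into the player and vanishes when something overlaps its sphere.
; On overlap it stores its start location and scale, then a timeline lerps it toward player pawn 0's current location while shrinking it and fading its point light.
; The actor destroys itself when the timeline finishes.
; The IsPawn player check is hard-wired to true with its comparison unconnected, so any overlapping actor triggers collection.
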(event `self.Sphere.OnComponentBeginOverlap`
  (params (OverlappedComponent :type "PrimitiveComponent Object Reference") (OtherActor :type "Actor Object Reference") (OtherComp :type "PrimitiveComponent Object Reference") (OtherBodyIndex :type Integer) (bFromSweep :type Boolean) (SweepResult :type "HitResult Structure (by ref)"))
  (`self.IsPawn` OtherActor
    (:`Is Player`
      (`self.SetStartValues`)
      (bind (_direction _locationintime _scaleintime _intensityintime) (`Timeline|TimelineCrystal`)
        (:`Update`
          (`self.CrystalLocation` _locationintime)
          (`self.CrystalScale` _scaleintime)
          (`self.CrystalIntensity` _intensityintime))
        (:`Finished`
          (`self.K2_DestroyActor`))))))

(fn `CrystalIntensity`
  (params (NewParam :type "Float (double-precision)"))
  (`LightComponent.SetIntensity` (`self.PointLight`) (`KismetMathLibrary.Lerp` (`self.LerpStartIntensity`) 0.0 NewParam)))

(fn `CrystalLocation`
  (params (Alpha :type "Float (double-precision)"))
  (`self.K2_SetActorLocation` (`KismetMathLibrary.VLerp` (`self.LerpStartLocation`) (`self.K2_GetActorLocation` (`GameplayStatics.GetPlayerPawn` 0)) Alpha)))

(fn `CrystalScale`
  (params (Alpha :type "Float (double-precision)"))
  (`self.SetActorScale3D` (`KismetMathLibrary.VLerp` (`self.LerpStartScale`) (0.0 0.0 0.0) Alpha)))

(fn `SetStartValues`
  (locals (LightIntensity :type "Float (double-precision)" :default 1.0))
  (set `self.LerpStartIntensity` 1.0)
  (set `self.LerpStartScale` (`self.GetActorScale3D`))
  (set `self.LerpStartLocation` (`self.K2_GetActorLocation`)))

(fn `UserConstructionScript`)