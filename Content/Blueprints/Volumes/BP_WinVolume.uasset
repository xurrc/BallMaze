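; BP_WinVolume is a level-exit volume that completes the level once no BP_crystal actors remain in it.
; Any actor overlap triggers the crystal count, printing a Polish "not all crystals collected" message if some are left.
; On completion it finds the current level in the LevelNames array and opens the next entry, or quits the game if it is the last.
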(event `self.ReceiveActorBeginOverlap`
  (params (OtherActor :type "Actor Object Reference"))
  (if (`self.CheckAnyCrystals` OtherActor)
    (`self.CompleteLevel` false)
    (else
      (`KismetSystemLibrary.PrintString` "Nie zebrales wszystkich krysztalow!"))))

(fn `CheckAnyCrystals`
  (params (OtherActor :type "Actor Object Reference"))
  (returns (ReturnValue :type Boolean))
  (bind _outactors (`GameplayStatics.GetAllActorsOfClass` "/Game/Blueprints/Collectibles/BP_crystal.BP_crystal_C"))
  (return (== 0 (`KismetArrayLibrary.Array_Length` _outactors))))

(fn `CheckLastIndex`
  (returns (ReturnValue :type Boolean))
  (return (== (`KismetArrayLibrary.Array_LastIndex` (`self.LevelNames`)) (`self.GetCurrentIndex`))))

(fn `CompleteLevel`
  (params (NewParam :type Boolean))
  (if (`self.CheckLastIndex`)
    (`KismetSystemLibrary.QuitGame` null "Quit")
    (else
      (`self.NextLevel`)))
  (return))

(fn `GetCurrentIndex`
  (returns (ReturnValue :type Integer))
  (bind _returnvalue (`GameplayStatics.GetCurrentLevelName` true))
  (return (`KismetArrayLibrary.Array_Find` (`self.LevelNames`) (`KismetStringLibrary.Conv_StringToName` _returnvalue))))

(fn `NextLevel`
  (`GameplayStatics.OpenLevel` (`|GetArrayItem` (`self.LevelNames`) (+ (`self.GetCurrentIndex`) 1))))

(fn `UserConstructionScript`)