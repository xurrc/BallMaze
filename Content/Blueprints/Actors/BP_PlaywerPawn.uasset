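; Player pawn that rolls a physics mesh by applying torque from movement axis input.
; On BeginPlay it fades the camera in and adds the health/damage widget to the screen.
; Damage subtracts from Health and prints it, while Tick checks for zero health to fade out and reload the current level.
; A ChangeCameraView function, not called within this Blueprint, sets spring arm length and rotation.
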(event `InputAxis|Move Forward/Backwards`
  (params (AxisValue :type "Float (single-precision)"))
  (`PrimitiveComponent.AddTorqueInRadians` (`self.StaticMesh`) (`KismetMathLibrary.MakeVector` 0.0 (* AxisValue (`self.Torque Strenght`))) "None" true))

(event `InputAxis|Move Left/Righ`
  (params (AxisValue :type "Float (single-precision)"))
  (`PrimitiveComponent.AddTorqueInRadians` (`self.StaticMesh`) (`KismetMathLibrary.MakeVector` (* AxisValue (`self.Torque Strenght`))) "None" true))

(event `self.ReceiveBeginPlay`
  ;[1 0.5021 0.939] LevelView Setup
  (`self.LevelFadeIn`)
  (`self.LevelUI`))

(event `self.ReceiveTick`
  (params (DeltaSeconds :type "Float (single-precision)"))
  ;[1 1 1] LevelRestartFromDamage
  (`self.LevelRestartByDeath`))

(event `self.ReceiveAnyDamage`
  (params (Damage :type "Float (single-precision)") (DamageType :type "DamageType Object Reference") (InstigatedBy :type "Controller Object Reference") (DamageCauser :type "Actor Object Reference"))
  ;[1 0.2332 0.1635] ApplyingDamage
  (`self.ApplyingDamage` Damage))

(fn `ApplyingDamage`
  (params (B :type "Float (double-precision)"))
  (bind _output_get (set `self.Health` (- (`self.Health`) B)))
  (`KismetSystemLibrary.PrintString` (`KismetStringLibrary.Conv_DoubleToString` _output_get) true true (struct :`G` 0.734375 :`B` 0.108742 :`A` 1.0) 0.2))

(fn `ChangeCameraView`
  (params (PitchSpringArm :type "Float (double-precision)") (`:enghtSproingArm` :type "Float (double-precision)") (Roll :type "Float (double-precision)"))
  (bind _springarm (`self.SpringArm`))
  (set `SpringArmComponent.TargetArmLength` `:enghtSproingArm` _springarm)
  (`SceneComponent.K2_SetWorldRotation` _springarm (`KismetMathLibrary.MakeRotator` Roll PitchSpringArm) false false))

(fn `LevelFadeIn`
  (`PlayerCameraManager.StartCameraFade` :`self` (`GameplayStatics.GetPlayerCameraManager` 0) :`FromAlpha` 1.0 :`Duration` 3.0))

(fn `LevelUI`
  (bind _returnvalue (`|CreateWidget` "/Game/Blueprints/Health_Damage_display.Health_Damage_display_C"))
  (`UserWidget.AddToPlayerScreen` _returnvalue 0))

(fn `UserConstructionScript`)